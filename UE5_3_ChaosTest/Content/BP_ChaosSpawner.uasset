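; Spawner actor that emits BP_ChaosPhysic bodies from its Arrow components and pools them into instance actors, apparently as a physics stress test.
; A Delay on Tick paces spawning round-robin through the arrows, pushing each body forward and printing the running total.
; Each body receives the spawner as its Pool; RequestPool adds a given actor's transform to the current BP_ChaosInstance, starting another when full or invalid.
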(event `self.ReceiveBeginPlay`
  (for _array_element (`self.K2_GetComponentsByClass` "/Script/Engine.ArrowComponent")
    (bind _asarrow_component (cast `ArrowComponent` _array_element))
    (`KismetArrayLibrary.Array_Add` (`self.Arrows`) _asarrow_component)))

(event `self.ReceiveTick`
  (params (DeltaSeconds :type "Float (single-precision)"))
  (bind _spawnerindex (`self.SpawnerIndex`))
  (bind _output (`|GetArrayItem` (`self.Arrows`) (`self.SpawnerIndex`)))
  (bind _returnvalue (* (`SceneComponent.GetForwardVector` _output) 20.0))
  (`KismetSystemLibrary.Delay` (`self.Speed`))
  (bind _returnvalue_2 (`|SpawnActorFromClass` "/Game/BP_ChaosPhysic.BP_ChaosPhysic_C" (`KismetMathLibrary.MakeTransform` (+ _returnvalue (`SceneComponent.K2_GetComponentLocation` _output)) (`SceneComponent.K2_GetComponentRotation` _output)) "AdjustIfPossibleButAlwaysSpawn" "MultiplyWithRoot" null self (`self.Nanite`) (`self.Optimize`) null))
  (`PrimitiveComponent.AddForce` (`StaticMeshActor.StaticMeshComponent` _returnvalue_2) _returnvalue "None" false)
  (`/Engine/EditorBlueprintResources/StandardMacros.IncrementInt` (`self.Total`)
    (:`  `
      (`/Engine/EditorBlueprintResources/StandardMacros.IncrementInt` _spawnerindex
        (:`  `
          (set `self.SpawnerIndex` (mod _spawnerindex (`KismetArrayLibrary.Array_Length` (`self.Arrows`))))
          (`KismetSystemLibrary.PrintString` (`KismetStringLibrary.Concat_StrStr` "Physic Actors: " (`KismetStringLibrary.Conv_IntToString` (`self.Total`))) true false (struct :`G` 0.66 :`B` 1.0 :`A` 1.0) 0.0))))))

(fn `RequestPool`
  (params (Actor :type "StaticMeshActor Object Reference"))
  (if (>= (`self.InstancePoolCount`) (`self.PerPoolActors`))
    (set `self.InstancePoolCount` 0)
    (bind _returnvalue (`|SpawnActorFromClass` "/Game/BP_ChaosInstance.BP_ChaosInstance_C" (`self.GetTransform` Actor) "Undefined" "MultiplyWithRoot" null (`StaticMeshComponent.StaticMesh` (`StaticMeshActor.StaticMeshComponent` Actor)) null :!label _label))
    (set `self.CurrentInstance` _returnvalue)
    (else
      (`/Engine/EditorBlueprintResources/StandardMacros.IsValid` (`self.CurrentInstance`)
        (:`Is Valid`
          _)
        (:`Is Not Valid`
          (goto _label)))))
  (`/Game/BP_ChaosInstance.AddInstanceLocation` (`self.CurrentInstance`) (`self.GetTransform` Actor))
  (`/Engine/EditorBlueprintResources/StandardMacros.IncrementInt` (`self.InstancePoolCount`)))

(fn `UserConstructionScript`)