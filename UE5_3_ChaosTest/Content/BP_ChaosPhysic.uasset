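; BP_ChaosPhysic is a small physics cube actor that stops simulating after a short lifetime, apparently to limit the cost of many physics objects.
; The construction script picks a Nanite or standard cube mesh from the Nanite flag.
; After a fixed delay from BeginPlay it disables physics; non-Nanite cubes with a valid Pool then pass themselves to RequestPool and destroy themselves.
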(event `self.ReceiveBeginPlay`
  (bind _pool (`self.Pool`))
  (`KismetSystemLibrary.Delay` 10.0)
  (`PrimitiveComponent.SetSimulatePhysics` (`self.StaticMeshComponent`) false)
  (if (not (`self.Nanite`))
    (`/Engine/EditorBlueprintResources/StandardMacros.IsValid` _pool
      (:`Is Valid`
        (`/Game/BP_ChaosSpawner.RequestPool` _pool self)
        (`self.K2_DestroyActor`)))))

(fn `UserConstructionScript`
  (`StaticMeshComponent.SetStaticMesh` (`self.StaticMeshComponent`) (select `bool` (`self.Nanite`) :`false` "/Game/Cube_Small.Cube_Small" :`true` "/Game/Cube_Small_Nanite.Cube_Small_Nanite" :!type "StaticMesh Object Reference")))