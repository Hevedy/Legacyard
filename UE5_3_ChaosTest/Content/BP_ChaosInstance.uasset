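; BP_ChaosInstance is an actor that renders many copies of one Model mesh through a hierarchical instanced static mesh component.
; The construction script assigns Model to the component when it is valid, and BeginPlay assigns it again.
; AddInstanceLocation lets a caller add an instance at a given world-space transform.
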(event `self.ReceiveBeginPlay`
  (`StaticMeshComponent.SetStaticMesh` (`self.HierarchicalInstancedStaticMesh`) (`self.Model`)))

(fn `AddInstanceLocation`
  (params (Transform :type "Transform Structure"))
  (`InstancedStaticMeshComponent.AddInstance` (`self.HierarchicalInstancedStaticMesh`) Transform true))

(fn `UserConstructionScript`
  (`/Engine/EditorBlueprintResources/StandardMacros.IsValid` (`self.Model`)
    (:`Is Valid`
      (`StaticMeshComponent.SetStaticMesh` (`self.HierarchicalInstancedStaticMesh`) (`self.Model`)))))