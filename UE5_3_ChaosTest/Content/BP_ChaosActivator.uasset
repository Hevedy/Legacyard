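; BP_ChaosActivator is a trigger actor that activates BP_ChaosPhysic objects entering its sphere.
; The construction script sizes the sphere from the Size variable.
; On overlap, it casts the other actor to BP_ChaosPhysic, calls Simulate, then applies PushForce from the sphere's location using Size as the radius.
; A cast to BP_ChaosInstance and a debug print are left unconnected.
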(event `self.Sphere.OnComponentBeginOverlap`
  (params (OverlappedComponent :type "PrimitiveComponent Object Reference") (OtherActor :type "Actor Object Reference") (OtherComp :type "PrimitiveComponent Object Reference") (OtherBodyIndex :type Integer) (bFromSweep :type Boolean) (SweepResult :type "HitResult Structure (by ref)"))
  (bind _asbp_chaos_physic (cast `/Game/BP_ChaosPhysic` OtherActor))
  (`/Game/BP_ChaosPhysic.Simulate` _asbp_chaos_physic)
  (`/Game/BP_ChaosPhysic.PushForce` _asbp_chaos_physic (`SceneComponent.K2_GetComponentLocation` (`self.Sphere`)) (`self.Size`)))

(fn `UserConstructionScript`
  (`SphereComponent.SetSphereRadius` (`self.Sphere`) (`self.Size`) true))